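; BP_WeaponSystem manages a third-person character's weapons: spawning, equipping, cycling and firing.
; On BeginPlay the server spawns a base weapon and a railgun, attaches them hidden to the weapon_r socket, and equips the first.
; A server event cycles CurrentWeapon through the list, while its RepNotify swaps visibility through a cached reference, calls OnEquip and signals the change.
; Fire delegates to the cached weapon, then signals the ammo change.
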(event Custom|EquipNextWeapon_Server
  (Variables|Default|SetCurrentWeapon (Utilities|Array|Get(acopy) (Variables|Default|GetWeaponList) (Math|Integer|%(Integer) (+ (Utilities|Array|FindItem (Variables|Default|GetWeaponList) (Variables|Default|GetCurrentWeapon)) 1) (Utilities|Array|Length (Variables|Default|GetWeaponList))))))

(event EventBeginPlay
  (bind _asbp_third_person_character (Utilities|Casting|CastToBP_ThirdPersonCharacter (Components|GetOwner)))
  (Variables|Default|SetAs%20BP%20Third%20Person%20Character _asbp_third_person_character)
  (if (Networking|IsServer)
    (CallFunction|SpawnWeapon "/Game/Weapons/BP_WeaponBase.BP_WeaponBase_C")
    (CallFunction|SpawnWeapon "/Game/Weapons/BP_Railgun.BP_Railgun_C")
    (Variables|Default|SetCurrentWeapon (Utilities|Array|Get(acopy) (Variables|Default|GetWeaponList)))))

(fn SpawnWeapon
  (params (Weapon :type BP%20Weapon%20Base%20Class%20Reference))
  (if (Ability|HasAuthority (Variables|Default|GetAs%20BP%20Third%20Person%20Character))
    (bind _returnvalue (Game|SpawnActorfromClass Weapon (Math|Transform|MakeTransform "0, 0, 0") "Undefined" "MultiplyWithRoot" (Variables|Default|GetAs%20BP%20Third%20Person%20Character) 0))
    (Transformation|AttachComponentToComponent _returnvalue (Variables|/Script/Engine.Character|GetMesh (Variables|Default|GetAs%20BP%20Third%20Person%20Character)) "weapon_r" "KeepRelative" "KeepRelative" "KeepRelative" true)
    (Rendering|SetActorHiddenInGame _returnvalue true)
    (Utilities|Array|Add (Variables|Default|GetWeaponList) _returnvalue)))

(fn Fire
  (params (TargetPoint :type Vector) (TargetActor :type Actor%20Object%20Reference))
  (bind _currentweaponcache (Variables|Default|GetCurrentWeaponCache))
  (Default|Fire _currentweaponcache TargetPoint TargetActor)
  (Default|CallOnAmmoCountChanged _currentweaponcache))

(fn OnRepCurrentWeapon
  (Utilities|FlowControl|Sequence
    (:then_0
      (Utilities|IsValid (Variables|Default|GetCurrentWeaponCache)
        (:Is%20Valid
          (Rendering|SetActorHiddenInGame (Variables|Default|GetCurrentWeaponCache) true))))
    (:then_1
      (bind _output_get (Variables|Default|SetCurrentWeaponCache (Variables|Default|GetCurrentWeapon)))
      (Rendering|SetActorHiddenInGame _output_get false)
      (Default|OnEquip _output_get)
      (Default|CallOnEquipWeapon _output_get))))