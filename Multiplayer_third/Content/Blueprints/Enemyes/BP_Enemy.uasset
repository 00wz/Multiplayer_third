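; BP_Enemy is an enemy character Blueprint that handles health, death and a self-explosion.
; Damage lowers Health only on the server and triggers Die at zero, which ragdolls the mesh, stops shooting and movement, disables capsule collision and sets a lifespan.
; Explode applies a radial blast using its radius, force and damage variables, then destroys the actor.
; Both Die and Explode call OnDead, and BeginPlay links unarmed animation layers.
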(event Custom|Die
  (CallFunction|ActiveRagdoll)
  (Variables|Default|SetIsShootingAllowed false)
  (Default|CallOnDead self)
  (Collision|SetCollisionEnabled (Variables|Default|GetCapsuleComponent) "NoCollision")
  (Actor|SetLifeSpan 1e+01))

(event Custom|Explode
  (CallFunction|Explode (Transformation|GetActorLocation) false (Variables|Default|GetExplodeRadius) (Variables|Default|GetMaxExplodeForce) (Variables|Default|GetMaxExplodeDamage))
  (Actor|DestroyActor)
  (Default|CallOnDead self))

(event EventDamage
  (params (value :type Float%20%28double-precision%29))
  (if (Networking|IsServer)
    (bind _output_get (Variables|Default|SetHealth (- (Variables|Default|GetHealth) value)))
    (if (<= _output_get 0.0)
      (CallFunction|Die))))

(event EventBeginPlay
  (Components|SkeletalMesh|AnimationBlueprintLinking|LinkAnimClassLayers (Variables|Character|GetMesh) "/Game/Characters/Heroes/Mannequin/Animations/Locomotion/Unarmed/ABP_UnarmedAnimLayers.ABP_UnarmedAnimLayers_C"))

(fn ConstructionScript)

(fn ActiveRagdoll
  (Physics|SetSimulatePhysics (Variables|Character|GetMesh) true)
  (Pawn|Components|CharacterMovement|DisableMovement (Variables|Character|GetCharacterMovement)))