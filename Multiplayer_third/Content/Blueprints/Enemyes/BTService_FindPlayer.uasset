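; Behavior tree service that finds the closest living player for an AI-controlled enemy.
; On activation, it scans the GameState PlayerArray for BP_ThirdPersonCharacter pawns that are not dead, comparing squared distances to the controlled pawn.
; It writes the nearest pawn to the Result blackboard key, or None when no player qualifies.
; The search runs only on activation, with no tick update.
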(event EventReceiveActivationAI
  (params (OwnerController :type AI%20Controller%20Object%20Reference) (ControlledPawn :type Pawn%20Object%20Reference))
  (Utilities|FlowControl|Sequence
    (:then_0
      (Variables|Default|SetClosestPlayer 0)
      (Variables|Default|SetDistanceToClosestPlayer (Class|MyBlueprintFunctionLibrary|MaxFloat))
      (for _array_element (Variables|/Script/Engine.GameStateBase|GetPlayerArray (Game|GetGameState))
        (bind _asbp_third_person_character (Utilities|Casting|CastToBP_ThirdPersonCharacter (PlayerState|GetPawn _array_element)))
        (if (not (Variables|/Game/Blueprints/BP_ThirdPersonCharacter.BP_ThirdPersonCharacter_C|GetIsDead _asbp_third_person_character))
          (if (< (Math|Vector|VectorLengthSquared (- (Transformation|GetActorLocation (PlayerState|GetPawn _array_element)) (Transformation|GetActorLocation ControlledPawn))) (Variables|Default|GetDistanceToClosestPlayer))
            (Variables|Default|SetDistanceToClosestPlayer (Math|Vector|VectorLengthSquared (- (Transformation|GetActorLocation (PlayerState|GetPawn _array_element)) (Transformation|GetActorLocation ControlledPawn))))
            (Variables|Default|SetClosestPlayer (PlayerState|GetPawn _array_element))))))
    (:then_1
      (Class|BTFunctionLibrary|SetBlackboardValueasObject (Variables|Default|GetResult) (Variables|Default|GetClosestPlayer)))))