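; Wave-based enemy spawner that starts a wave on BeginPlay and grows each following wave by one enemy.
; While enabled, each wave spawns enemies one by one at a timed interval, with the server placing BP_Enemy actors at random spawn points.
; Each enemy's death event is bound to remove it from the tracked list, and an empty list starts the next wave.
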(event Custom|StartEnemyWave
  (if (Variables|Default|GetIsEnable)
    (for _index (range 1 (Variables|Default|GetWaveEnemyCount))
      (CallFunction|SpawnEnemy)
      (Utilities|FlowControl|Delay (Variables|Default|GetSpawnTimeInterval)))
    (CallFunction|IncreaseComplexity)))

(event EventBeginPlay
  (CallFunction|StartEnemyWave))

(fn ConstructionScript)

(fn SpawnEnemy
  (if (Networking|IsServer)
    (bind _returnvalue (Game|SpawnActorfromClass "/Game/Blueprints/Enemyes/BP_Enemy.BP_Enemy_C" (Transformation|GetActorTransform (.OutItem (Utilities|Array|Random (Variables|Default|GetSpawnPoints)))) "Undefined" "MultiplyWithRoot" 0 0))
    (Utilities|Array|Add (Variables|Default|GetEnemyes) _returnvalue)
    (EventDispatchers|BindEventtoOnDead _returnvalue (EventDispatchers|CreateEvent :!event OnEnemyDead))))

(fn OnEnemyDead
  (params (sender :type BP%20Enemy%20Object%20Reference))
  (Utilities|Array|RemoveItem (Variables|Default|GetEnemyes) sender)
  (CallFunction|CheckEnemyes))

(fn CheckEnemyes
  (if (Utilities|Array|IsEmpty (Variables|Default|GetEnemyes))
    (CallFunction|StartEnemyWave)))

(fn IncreaseComplexity
  (Math|Integer|IncrementInt (Variables|Default|GetWaveEnemyCount)))