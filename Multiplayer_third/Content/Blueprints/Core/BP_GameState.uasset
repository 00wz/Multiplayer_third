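; BP_GameState is a game state Blueprint that shows UI for game-over and traveling events.
; On game over, it creates a W_GameOver widget, fills its total time text with the server world time as a timespan, and adds it to the viewport.
; On traveling, it creates a W_TrevelingLabel widget and adds it to the viewport.
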(event Custom|OnGameOverEvent
  (bind _returnvalue (UserInterface|CreateWidget "/Game/Blueprints/UI/W_GameOver.W_GameOver_C"))
  (Rendering|Components|TextRender|SetText (Variables|/Game/Blueprints/UI/W_GameOver.W_GameOver_C|GetTotalTimeText _returnvalue) (Class|KismetTextLibrary|AsTimespanTimespan (Math|Timespan|FromSeconds (GameState|GetServerWorldTimeSeconds (Game|GetGameState)))))
  (UserInterface|Viewport|AddtoViewport _returnvalue 0))

(event Custom|OnTrevelingEvent
  (bind _returnvalue (UserInterface|CreateWidget "/Game/Blueprints/UI/W_TrevelingLabel.W_TrevelingLabel_C"))
  (UserInterface|Viewport|AddtoViewport _returnvalue 0))

(fn ConstructionScript)