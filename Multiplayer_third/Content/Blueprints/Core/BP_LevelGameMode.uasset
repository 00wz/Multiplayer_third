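; BP_LevelGameMode is a level game mode that ends and restarts the match once every player is dead.
; On each player death it checks the dead flag on every BP_GamePlayerState in the game state's player array.
; When all are dead, it fires the game-over event on BP_GameState, waits briefly, fires its traveling event, then has BP_GameInstance restart the match.
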(event Custom|OnGameOver
  (bind _asbp_game_state (Utilities|Casting|CastToBP_GameState (Game|GetGameState)))
  (Default|OnGameOverevent _asbp_game_state)
  (Utilities|FlowControl|Delay 1.0)
  (Default|OnTrevelingEvent _asbp_game_state)
  (bind _asbp_game_instance (Utilities|Casting|CastToBP_GameInstance (Game|GetGameInstance)))
  (Default|RestartMatch _asbp_game_instance))

(event EventOnPlayerDead
  (params (sender :type BP%20Game%20Player%20State%20Object%20Reference))
  (bind _allplayersaredead (CallFunction|CheckPlayers))
  (if _allplayersaredead
    (CallFunction|OnGameOver)))

(fn ConstructionScript)

(fn CheckPlayers
  (for _array_element (Variables|/Script/Engine.GameStateBase|GetPlayerArray (Game|GetGameState))
    (bind _asbp_game_player_state (Utilities|Casting|CastToBP_GamePlayerState _array_element))
    (if (not (Variables|/Game/Blueprints/Core/BP_GamePlayerState.BP_GamePlayerState_C|GetIsDead _asbp_game_player_state))
      (return false)))
  (return true))