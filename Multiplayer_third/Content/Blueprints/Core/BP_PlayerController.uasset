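; Player controller that creates the HUD and pause menu for the local player and forwards fire, jump and weapon-switch calls to the third-person character.
; Character events update weapon icon, ammo and health or hide the game panel on death, while a looping timer shows server time.
; Pausing only toggles menu visibility and input mode, without stopping the game.
; Exit destroys the session through the game instance and opens the lobby map.
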(event Custom|TogglePause
  (if (Variables|Default|GetIsPause)
    (Variables|Default|SetIsPause false)
    (Input|SetInputModeGameOnly self false)
    (Widget|SetVisibility (Variables|Default|GetPauseMenu) "Hidden")
    (else
      (Variables|Default|SetIsPause true)
      (Input|SetInputModeUIOnly self (Variables|Default|GetPauseMenu) "DoNotLock" false)
      (Widget|SetVisibility (Variables|Default|GetPauseMenu) "Visible"))))

(event Custom|CustomEvent_0
  (params (Sender :type BP%20Weapon%20Base%20Object%20Reference))
  (CallFunction|RefreshHudAmmo Sender))

(event Custom|CustomEvent
  (params (Weapon :type BP%20Weapon%20Base%20Object%20Reference))
  (CallFunction|RefreshHudWeapon Weapon)
  (CallFunction|RefreshHudAmmo Weapon))

(event Custom|CustomEvent_1
  (params (HealthRatio :type Float%20%28double-precision%29))
  (CallFunction|RefreshHudHealth HealthRatio))

(event Custom|EquipNextWeapon
  (Default|EquipNextWeapon (Variables|Default|GetPlayerCharacter)))

(event Custom|Fire
  (Default|Fire (Variables|Default|GetPlayerCharacter)))

(event Custom|CustomEvent_2
  (Default|HideGamePanel (Variables|Default|GetHUD)))

(event Custom|Jump
  (Character|Jump (Variables|Default|GetPlayerCharacter)))

(event EventBeginPlay
  (if (Pawn|IsLocalPlayerController)
    (Utilities|FlowControl|Sequence
      (:then_0
        (bind _returnvalue (UserInterface|CreateWidget "/Game/Blueprints/UI/W_HUD.W_HUD_C" self))
        (bind _output_get (Variables|Default|SetHUD _returnvalue))
        (UserInterface|Viewport|AddtoViewport _output_get 0))
      (:then_1
        (bind _returnvalue_2 (UserInterface|CreateWidget "/Game/Blueprints/UI/W_Pause.W_Pause_C" self))
        (bind _output_get_2 (Variables|Default|SetPauseMenu _returnvalue_2))
        (UserInterface|Viewport|AddtoViewport _output_get_2 0)
        (Widget|SetVisibility _output_get_2 "Hidden")
        (EventDispatchers|BindEventtoOnClicked (Variables|/Game/Blueprints/UI/W_Pause.W_Pause_C|GetResumeButton _output_get_2) (EventDispatchers|CreateEvent :!event Custom|TogglePause))
        (EventDispatchers|BindEventtoOnClicked (Variables|/Game/Blueprints/UI/W_Pause.W_Pause_C|GetExitButton _output_get_2) (EventDispatchers|CreateEvent :!event Exit)))
      (:then_2
        (bind _asbp_third_person_character (Utilities|Casting|CastToBP_ThirdPersonCharacter (Pawn|GetControlledPawn)))
        (bind _output_get_3 (Variables|Default|SetPlayerCharacter _asbp_third_person_character))
        (EventDispatchers|BindEventtoOnWeaponEquip _output_get_3 (delegate Custom|CustomEvent))
        (EventDispatchers|BindEventtoOnAmmoCountChanged _output_get_3 (delegate Custom|CustomEvent_0))
        (EventDispatchers|BindEventtoOnHealthChanged _output_get_3 (delegate Custom|CustomEvent_1))
        (EventDispatchers|BindEventtoOnDie _output_get_3 (delegate Custom|CustomEvent_2)))
      (:then_3
        (Utilities|Time|SetTimerbyFunctionName 0 "RefreshHudGameTime" 1.0 true))
      (:then_4
        (Input|SetInputModeGameOnly self false)))))

(event Input|ActionEvents|InputActionPause
  (params (Key :type Key%20Structure :default "None"))
  (:Pressed
    (CallFunction|TogglePause)))

(fn ConstructionScript)

(fn Exit
  (bind _asbp_game_instance (Utilities|Casting|CastToBP_GameInstance (Game|GetGameInstance)))
  (Default|DestroySession _asbp_game_instance)
  (Game|OpenLevel(byObjectReference) "/Game/Maps/LobbyMap.LobbyMap"))

(fn RefreshHudWeapon
  (params (Weapon :type BP%20Weapon%20Base%20Object%20Reference))
  (Appearance|SetBrushfromTexture (Variables|/Game/Blueprints/UI/W_HUD.W_HUD_C|GetWeaponIcon (Variables|Default|GetHUD)) (Variables|/Game/Weapons/BP_WeaponBase.BP_WeaponBase_C|GetIcon Weapon) false))

(fn RefreshHudAmmo
  (params (Weapon :type BP%20Weapon%20Base%20Object%20Reference))
  (bind _hud (Variables|Default|GetHUD))
  (bind _ammo (Variables|/Game/Weapons/BP_WeaponBase.BP_WeaponBase_C|GetAmmo Weapon))
  (bind _ammunitionquantity (Variables|/Game/Blueprints/UI/W_HUD.W_HUD_C|GetAmmunitionQuantity _hud))
  (if (!= (Class|MyBlueprintFunctionLibrary|MaxInt) _ammo)
    (Variables|/Script/UMG.TextBlock|SetText _ammunitionquantity (Utilities|Text|ToText(Integer) _ammo))
    (else
      (Variables|/Script/UMG.TextBlock|SetText _ammunitionquantity "inf"))))

(fn RefreshHudHealth
  (params (HealthRatio :type Float%20%28double-precision%29))
  (Variables|/Script/UMG.TextBlock|SetText (Variables|/Game/Blueprints/UI/W_HUD.W_HUD_C|GetHealthRatio (Variables|Default|GetHUD)) (Utilities|Text|ToText(Float) HealthRatio "HalfToEven" false true 1 324 0 0)))

(fn RefreshHudGameTime
  (Variables|/Script/UMG.TextBlock|SetText (Variables|/Game/Blueprints/UI/W_HUD.W_HUD_C|GetGameTime (Variables|Default|GetHUD)) (Class|KismetTextLibrary|AsTimespanTimespan (Math|Timespan|FromSeconds (GameState|GetServerWorldTimeSeconds (Game|GetGameState))))))