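; Base projectile actor for weapons that damages what it hits and expires after a short lifespan if it hits nothing.
; On hit, it passes its Damage value to any actor implementing the BI_IDamageble interface.
; Every hit, damageable or not, then spawns a concrete impact Niagara system and destroys the projectile.
; HitEffect feeds the hit location and normal to that system through Niagara user array parameters.
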(event EventBeginPlay
  (Actor|SetLifeSpan 1.0))

(event Collision|EventHit
  (params (MyComp :type Primitive%20Component%20Object%20Reference) (Other :type Actor%20Object%20Reference) (OtherComp :type Primitive%20Component%20Object%20Reference) (bSelfMoved :type Boolean) (HitLocation :type Vector :default "0, 0, 0") (HitNormal :type Vector :default "0, 0, 0") (NormalImpulse :type Vector :default "0, 0, 0") (Hit :type Hit%20Result%20Structure%20%28by%20ref%29))
  (Utilities|FlowControl|Sequence
    (:then_0
      (bind _asbi_idamageble (Utilities|Casting|CastToBI_IDamageble Other))
      (Default|Damage _asbi_idamageble (Variables|Default|GetDamage)))
    (:then_1
      (CallFunction|HitEffect HitLocation HitNormal)
      (Actor|DestroyActor))))

(fn ConstructionScript)

(fn HitEffect
  (params (Location :type Vector) (Normal :type Vector))
  (bind _returnvalue (Niagara|SpawnSystematLocation "/Game/Effects/Particles/Impacts/NS_ImpactConcrete.NS_ImpactConcrete" Location))
  (Class|NiagaraDataInterfaceArrayFunctionLibrary|SetNiagaraArrayPosition _returnvalue "User.ImpactPositions" (Utilities|Array|MakeArray Location))
  (Class|NiagaraDataInterfaceArrayFunctionLibrary|SetNiagaraArrayVector _returnvalue "User.ImpactNormals" (Utilities|Array|MakeArray Normal)))