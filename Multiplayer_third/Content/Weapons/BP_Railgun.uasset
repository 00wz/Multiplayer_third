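; Railgun weapon Blueprint that overrides its parent's firing functions to add ammo-limited shots with a Niagara tracer.
; Fire calls the parent version only while ammo remains; FireLogic decrements ammo, broadcasts the count change and sends damage to the target actor on the server only.
; FireEffect spawns an attached tracer at the Muzzle socket and passes the target point through a Niagara array parameter.
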(event EventBeginPlay
  (|CallParentFunction) ; This node is disabled and will not be called.\nDrag off pins to build functionality.
)

(event Collision|EventActorBeginOverlap
  (params (OtherActor :type Actor%20Object%20Reference)))

(event EventTick
  (params (DeltaSeconds :type Float%20%28single-precision%29)))

(fn ConstructionScript
  (|CallParentFunction))

(fn FireEffect
  (params (TargetPoint :type Vector :default "0, 0, 0"))
  (bind _returnvalue (Niagara|SpawnSystemAttached (Variables|Default|GetTracerSystem) (Variables|Default|GetDefaultSceneRoot) "None" (.location (Transformation|GetSocketTransform (Variables|Default|GetSkeletalMesh) "Muzzle" "RTS_Actor")) (Math|Rotator|MakeRotator 0.0 0.0 9e+01) "KeepRelativeOffset" true))
  (Class|NiagaraComponent|SetVariableBool _returnvalue "User.Trigger" true)
  (Class|NiagaraDataInterfaceArrayFunctionLibrary|SetNiagaraArrayVector _returnvalue "User.ImpactPositions" (Utilities|Array|MakeArray TargetPoint)))

(fn FireLogic
  (params (FireDirection :type Vector :default "0, 0, 0") (TargetActor :type Actor%20Object%20Reference))
  (Math|Integer|DecrementInt (Variables|Default|GetAmmo)
    (:%20%20
      (Default|CallOnAmmoCountChanged self)
      (if (Networking|IsServer)
        (Class|BIIDamageble|Damage(Message) TargetActor (Variables|Default|GetDamage))))))

(fn Fire
  (params (TargetPoint :type Vector :default "0, 0, 0") (TargetActor :type Actor%20Object%20Reference))
  (if (> (Variables|Default|GetAmmo) 0)
    (|CallParentFunction TargetPoint TargetActor)))