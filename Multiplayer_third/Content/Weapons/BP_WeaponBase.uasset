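; Base weapon actor for the third-person character, handling equip animation layers, firing and fire replication.
; Init caches the owning character and its anim instance, and OnEquip links the weapon's anim layer.
; Fire runs locally first, playing weapon and character animations, muzzle Niagara and spawning a projectile toward the target point.
; It then relays through a server event to non-owning clients, which repeat both visuals and projectile spawn locally.
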(event Custom|Fire_OtherClients
  (params (FireDirection :type Vector) (TargetPoint :type Vector) (TargetActor :type Actor%20Object%20Reference))
  (if (not (Class|MyBlueprintFunctionLibrary|HasLocalNetOwner self))
    (CallFunction|ShowFire TargetPoint)
    (CallFunction|FireLogic FireDirection TargetActor)))

(event Custom|Fire_Server
  (params (FireDirection :type Vector) (TargetPoint :type Vector) (TargetActor :type Actor%20Object%20Reference))
  (CallFunction|FireOtherClients FireDirection TargetPoint TargetActor))

(event Custom|OnEquip
  (Utilities|FlowControl|Sequence
    (:then_0
      (if (not (Variables|Default|GetIsInitialize))
        (CallFunction|Init)))
    (:then_1
      (Components|SkeletalMesh|AnimationBlueprintLinking|LinkAnimClassLayers (Variables|/Script/Engine.Character|GetMesh (Variables|Default|GetAs%20BP%20Third%20Person%20Character_0)) (Variables|Default|GetAnimLayer)))))

(event Custom|Init
  (bind _asbp_third_person_character (Utilities|Casting|CastToBP_ThirdPersonCharacter (Components|GetOwner)))
  (Variables|Default|SetAs%20BP%20Third%20Person%20Character_0 _asbp_third_person_character)
  (bind _asabp_mannequin_base (Utilities|Casting|CastToABP_Mannequin_Base (Components|SkeletalMesh|GetAnimInstance (Variables|/Script/Engine.Character|GetMesh _asbp_third_person_character))))
  (Variables|Default|SetCharacterAnimInstance _asabp_mannequin_base)
  (Variables|Default|SetIsInitialize true))

(event EventBeginPlay
  (if (not (Variables|Default|GetIsInitialize))
    (CallFunction|Init)))

(fn ConstructionScript)

(fn ShowFire
  (params (TargetPoint :type Vector))
  (CallFunction|FireAnimationPlay)
  (CallFunction|FireEffect TargetPoint))

(fn Fire
  (params (TargetPoint :type Vector) (TargetActor :type Actor%20Object%20Reference))
  (bind _arrow (Variables|Default|GetArrow))
  (bind _returnvalue (Transformation|GetWorldLocation _arrow))
  (bind _returnvalue_2 (- TargetPoint _returnvalue))
  (Utilities|FlowControl|Sequence
    (:then_0
      (CallFunction|ShowFire TargetPoint)
      (CallFunction|FireLogic _returnvalue_2 TargetActor))
    (:then_1
      (CallFunction|FireServer _returnvalue_2 TargetPoint TargetActor))))

(fn FireEffect
  (params (TargetPoint :type Vector))
  (bind _skeletalmesh (Variables|Default|GetSkeletalMesh))
  (bind _returnvalue (Transformation|GetSocketTransform _skeletalmesh "Muzzle" "RTS_World"))
  (bind _returnvalue_2 (Niagara|SpawnSystematLocation "/Game/Effects/Particles/Weapons/NS_WeaponFire.NS_WeaponFire" (.location _returnvalue) (.rotation _returnvalue)))
  (Class|NiagaraComponent|SetVariableBool _returnvalue_2 "User.Trigger" true)
  (Niagara|SetNiagaraVariable(Vector3) _returnvalue_2 "User.Direction" (Math|Vector|GetForwardVector (.rotation _returnvalue))))

(fn FireAnimationPlay
  (Class|AnimInstance|PlaySlotAnimationasDynamicMontage (Components|SkeletalMesh|GetAnimInstance (Variables|Default|GetSkeletalMesh)) (Variables|Default|GetFireWeaponSequence) "DefaultSlot" 0.0 0.0 1.0 1 -1.0 0.0)
  (Class|AnimInstance|MontagePlaywithBlendin (Variables|Default|GetCharacterAnimInstance) (Variables|Default|GetFireCharacterAnimationMontage) (Utilities|Struct|MakeAlphaBlendArgs 0 0.05 "Linear") 1.0 "MontageLength" 0.0 true)
  (Variables|/Game/Characters/Heroes/Mannequin/Animations/ABP_Mannequin_Base.ABP_Mannequin_Base_C|SetTimeSinceFiredWeapon (Variables|Default|GetCharacterAnimInstance) 0.0))

(fn FireLogic
  (params (FireDirection :type Vector) (TargetActor :type Actor%20Object%20Reference))
  (Game|SpawnActorfromClass "/Game/Weapons/BP_ProjectileBase.BP_ProjectileBase_C" (Math|Transform|MakeTransform (Transformation|GetWorldLocation (Variables|Default|GetArrow)) (Math|Rotator|FindLookatRotation (Math|Vector|VectorZero) FireDirection)) "Undefined" "MultiplyWithRoot" 0 0))